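; Pig enemy character that chases the player and deals melee damage, with a health widget fed from its own health.
; BeginPlay and pawn sensing trigger FollowPlayer, whose AI MoveTo success runs a jump attack using a sphere overlap and cooldown.
; Damage spawns blood and updates the widget; death awards player score, disables collision, plays effects and sound, then launches the body skyward before destroying it.
; Tick is disabled at BeginPlay.
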(event `self.ReceiveBeginPlay`
  (`NiagaraFunctionLibrary.SpawnSystemAttached` "/Game/Vefects/Zap_VFX/VFX/Zap/Particles/NS_Zap_01_Red.NS_Zap_01_Red" (`self.Niagara`) "None" (0.0 0.0 0.0) (struct) "KeepRelativeOffset")
  (`GameplayStatics.PlaySoundAtLocation` "/Game/Vefects/Zap_VFX/Audio/SFX_Vefects_Zap_Small_01_Cue.SFX_Vefects_Zap_Small_01_Cue" (`SceneComponent.K2_GetComponentLocation` (`self.Sphere`)) (struct) 1.0 1.0 0.0 null null null null)
  (`self.SetActorTickEnabled` false)
  (bind _asbp_enemy (cast `/Game/Main/UI/BP_Enemy` (`WidgetComponent.GetUserWidgetObject` (`self.Widget1`))))
  (bind _output_get (set `self.As BP Enemy` _asbp_enemy))
  (set `/Game/Main/UI/BP_Enemy.CurrentHealthInt` (`self.CurrenHealth`) _output_get)
  (set `/Game/Main/UI/BP_Enemy.MaxHealth` (`self.MaxHealth`) _output_get)
  (set `self.isSeeingPlayer` true)
  (`self.FollowPlayer`))

(event `self.ReceiveAnyDamage`
  (params (Damage :type "Float (single-precision)") (DamageType :type "DamageType Object Reference") (InstigatedBy :type "Controller Object Reference") (DamageCauser :type "Actor Object Reference"))
  (`KismetSystemLibrary.PrintString` (`KismetStringLibrary.Conv_DoubleToString` 0.0))
  (`NiagaraFunctionLibrary.SpawnSystemAttached` "/Game/Main/Effects/BloodSplater1.BloodSplater1" (`self.CapsuleComponent`) "None" (0.0 0.0 0.0) (struct) "KeepRelativeOffset")
  (bind _output_get (set `self.CurrenHealth` (`KismetMathLibrary.FTrunc` (- (`self.CurrenHealth`) Damage))))
  (`/Game/Main/UI/BP_Enemy.Update heath` (`self.As BP Enemy`) _output_get)
  (if (<= _output_get 0)
    (set `self.isSeeingPlayer` false)
    (`NiagaraFunctionLibrary.SpawnSystemAttached` "/Game/Main/Effects/BloodSplater.BloodSplater" (`self.CapsuleComponent`) "None" (0.0 0.0 0.0) (struct) "KeepRelativeOffset")
    (bind _asbp_first_person_character (cast `/Game/FirstPerson/Blueprints/BP_FirstPersonCharacter` (`GameplayStatics.GetPlayerCharacter` 0)))
    (set `/Game/FirstPerson/Blueprints/BP_FirstPersonCharacter.Score` (+ (`/Game/FirstPerson/Blueprints/BP_FirstPersonCharacter.Score` _asbp_first_person_character) 750) _asbp_first_person_character)
    (`SkeletalMeshComponent.PlayAnimation` (`self.Mesh`) "/Game/Main/Animals/Cow/Armature_Death.Armature_Death" false)
    (`PrimitiveComponent.SetCollisionEnabled` (`self.CapsuleComponent`) "NoCollision")
    (`PrimitiveComponent.SetCollisionEnabled` (`self.Sphere`) "NoCollision")
    (`KismetSystemLibrary.Delay` 1.5)
    (`NiagaraFunctionLibrary.SpawnSystemAttached` "/Game/MixedVFX/Particles/Mix/NS_HealingAura.NS_HealingAura" (`self.Niagara`) "None" (0.0 0.0 0.0) (struct) "KeepRelativeOffset")
    (`KismetSystemLibrary.Delay` 1.5)
    (`GameplayStatics.SpawnSoundAttached` "/Game/MAX/Thurston_the_cat_m_e_m_e_-_www_youtube_com__www_ymate_cc_.Thurston_the_cat_m_e_m_e_-_www_youtube_com__www_ymate_cc_" (`self.Sphere`) "None" (0.0 0.0 0.0) (struct) "KeepRelativeOffset" false 1.0 1.0 0.0 null null)
    (`self.LaunchCharacter` (0.0 0.0 10000.0) false true)
    (`KismetSystemLibrary.Delay` 20.0)
    (`self.K2_DestroyActor`)))

(event `self.ReceiveTick`
  (params (DeltaSeconds :type "Float (single-precision)"))
  (`KismetSystemLibrary.PrintString` "tickers")
  (if (<= (`self.CurrenHealth`) 0)
    (set `self.isSeeingPlayer` false)
    (else
      (set `self.isSeeingPlayer` true)
      (`self.FollowPlayer`))))

(event `FollowPlayer`
  (if (`self.isSeeingPlayer`)
    (if (not (<= (`self.CurrenHealth`) 0))
      (`SkeletalMeshComponent.PlayAnimation` (`self.Mesh`) "/Game/Main/Animals/Cow/Armature_Run.Armature_Run" false)
      (`|AIMoveTo` self (0.0 0.0 0.0) (`GameplayStatics.GetPlayerCharacter` 0)
        (:`OnSuccess`
          (if (`self.canAttack?`)
            (set `self.canAttack?` false)
            (`SkeletalMeshComponent.PlayAnimation` (`self.Mesh`) "/Game/Main/Animals/Cow/Armature_Jump.Armature_Jump" false)
            (bind _outactors (`KismetSystemLibrary.SphereOverlapActors` (`SceneComponent.K2_GetComponentLocation` (`self.Arrow1`)) 10.0 (`self.Object Types`)))
            (for _array_element _outactors
              (if (`self.ActorHasTag` _array_element "Player")
                (`GameplayStatics.ApplyDamage` _array_element 40.0)))
            (`KismetSystemLibrary.Delay` 1.0)
            (set `self.canAttack?` true)
            (if (<= (`self.CurrenHealth`) 0)
              (set `self.isSeeingPlayer` false)
              (`|AIMoveTo` self (`KismetMathLibrary.Conv_DoubleToVector` (`SkeletalMeshComponent.GetPosition` (`self.Mesh`))) self))))))))

(event `self.PawnSensing.OnSeePawn`
  (params (Pawn :type "Pawn Object Reference"))
  (if (<= (`self.CurrenHealth`) 0)
    (`KismetSystemLibrary.PrintString` "im ded")
    (set `self.isSeeingPlayer` false)
    (`|AIMoveTo` self (`KismetMathLibrary.Conv_DoubleToVector` (`SkeletalMeshComponent.GetPosition` (`self.Mesh`))) self)
    (else
      (set `self.isSeeingPlayer` true)
      (`KismetSystemLibrary.PrintString` "isee you")
      (`self.FollowPlayer`)
      (`SkeletalMeshComponent.PlayAnimation` (`self.Mesh`) "/Game/Main/Animals/Cow/Armature_Run.Armature_Run" true)
      (if (not (`self.isSeeingPlayer`))
        (`SkeletalMeshComponent.PlayAnimation` (`self.Mesh`) "/Game/Main/Animals/Cow/Armature_Idle.Armature_Idle" false)))))

(fn `UserConstructionScript`)