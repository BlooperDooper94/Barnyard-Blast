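; Spawner actor that populates the area around its billboard with randomly chosen cow, pig or chicken AI running BT_Spawns.
; BeginPlay waits briefly, enables tick and spawns one animal; each tick spawns another within a wider square offset.
; Each tick shortens the tick interval down to a clamped minimum, so spawning accelerates.
; Random rolls repeat per check, skewing animal odds and making debug prints differ from actual results.
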(event `self.ReceiveBeginPlay`
  (bind _returnvalue (`KismetMathLibrary.RandomIntegerInRange` -1000 1000))
  (bind _returnvalue_2 (`KismetMathLibrary.RandomInteger` 2))
  (bind _returnvalue_3 (`KismetMathLibrary.RandomIntegerInRange` -1000 1000))
  (bind _returnvalue_4 (`KismetMathLibrary.RandomIntegerInRange` -1000 1000))
  (bind _returnvalue_5 (+ (`SceneComponent.K2_GetComponentLocation` (`self.Billboard`)) (`KismetMathLibrary.MakeVector` (`KismetMathLibrary.Conv_IntToDouble` _returnvalue_3) (`KismetMathLibrary.Conv_IntToDouble` _returnvalue_3))))
  (bind _returnvalue_6 (+ (`SceneComponent.K2_GetComponentLocation` (`self.Billboard`)) (`KismetMathLibrary.MakeVector` (`KismetMathLibrary.Conv_IntToDouble` _returnvalue_4) (`KismetMathLibrary.Conv_IntToDouble` _returnvalue_4))))
  (bind _returnvalue_7 (+ (`SceneComponent.K2_GetComponentLocation` (`self.Billboard`)) (`KismetMathLibrary.MakeVector` (`KismetMathLibrary.Conv_IntToDouble` _returnvalue) (`KismetMathLibrary.Conv_IntToDouble` _returnvalue))))
  (`KismetSystemLibrary.Delay` 5.0)
  (`self.SetActorTickEnabled` true)
  (`KismetSystemLibrary.PrintString` (`KismetStringLibrary.Conv_IntToString` _returnvalue_2))
  (if (== _returnvalue_2 0)
    (`AIBlueprintHelperLibrary.SpawnAIFromClass` "/Game/Main/Blueprint/BP_Cow.BP_Cow_C" "/Game/Main/Blueprint/BT_Spawns.BT_Spawns" _returnvalue_7 (struct) false null)
    (`KismetSystemLibrary.PrintString` (`KismetStringLibrary.Conv_VectorToString` _returnvalue_7))
    (`self.SetActorTickEnabled` true)
    (elif (== _returnvalue_2 1)
      (`AIBlueprintHelperLibrary.SpawnAIFromClass` "/Game/Main/Blueprint/BP_Pig.BP_Pig_C" "/Game/Main/Blueprint/BT_Spawns.BT_Spawns" _returnvalue_5 (struct) false null)
      (`KismetSystemLibrary.PrintString` (`KismetStringLibrary.Conv_VectorToString` _returnvalue_5))
      (`self.SetActorTickEnabled` true)
      (else
        (`AIBlueprintHelperLibrary.SpawnAIFromClass` "/Game/Main/Blueprint/BP_Chicken.BP_Chicken_C" "/Game/Main/Blueprint/BT_Spawns.BT_Spawns" _returnvalue_6 (struct) false null)
        (`KismetSystemLibrary.PrintString` (`KismetStringLibrary.Conv_VectorToString` _returnvalue_6))
        (`self.SetActorTickEnabled` true)))))

(event `self.ReceiveTick`
  (params (DeltaSeconds :type "Float (single-precision)"))
  (bind _returnvalue (`KismetMathLibrary.RandomInteger` 3))
  (bind _returnvalue_2 (+ (`SceneComponent.K2_GetComponentLocation` (`self.Billboard`)) (`KismetMathLibrary.MakeVector` (`KismetMathLibrary.Conv_IntToDouble` (`KismetMathLibrary.RandomIntegerInRange` -2000 2000)) (`KismetMathLibrary.Conv_IntToDouble` (`KismetMathLibrary.RandomIntegerInRange` -2000 2000)))))
  (`KismetSystemLibrary.PrintString` (`KismetStringLibrary.Conv_IntToString` _returnvalue))
  (if (== _returnvalue 1)
    (`AIBlueprintHelperLibrary.SpawnAIFromClass` "/Game/Main/Blueprint/BP_Cow.BP_Cow_C" "/Game/Main/Blueprint/BT_Spawns.BT_Spawns" _returnvalue_2 (struct) false null)
    (`KismetSystemLibrary.PrintString` (`KismetStringLibrary.Conv_VectorToString` _returnvalue_2))
    (`self.SetActorTickInterval` (`KismetMathLibrary.FClamp` (- (`self.GetActorTickInterval`) 0.1) 0.5 6.0))
    (elif (== _returnvalue 2)
      (`AIBlueprintHelperLibrary.SpawnAIFromClass` "/Game/Main/Blueprint/BP_Pig.BP_Pig_C" "/Game/Main/Blueprint/BT_Spawns.BT_Spawns" _returnvalue_2 (struct) false null)
      (`self.SetActorTickInterval` (`KismetMathLibrary.FClamp` (- (`self.GetActorTickInterval`) 0.1) 0.5 6.0))
      (else
        (`AIBlueprintHelperLibrary.SpawnAIFromClass` "/Game/Main/Blueprint/BP_Chicken.BP_Chicken_C" "/Game/Main/Blueprint/BT_Spawns.BT_Spawns" _returnvalue_2 (struct) false null)
        (`self.SetActorTickInterval` (`KismetMathLibrary.FClamp` (- (`self.GetActorTickInterval`) 0.1) 0.5 6.0))))))

(fn `UserConstructionScript`)