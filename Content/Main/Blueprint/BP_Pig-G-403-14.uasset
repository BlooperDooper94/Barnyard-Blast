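; Pig enemy pawn that chases the player character and dies when damage empties its health.
; BeginPlay disables tick, seeds a BP_Enemy health widget and starts an AIMoveTo chase, which pawn sensing re-triggers along with the run animation.
; Damage updates the widget; at zero health it stops the chase flag, spawns attached fire, plays the death animation, disables sphere collision and destroys the actor after a delay.
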(event `self.ReceiveBeginPlay`
  (`self.SetActorTickEnabled` false)
  (bind _asbp_enemy (cast `/Game/Main/UI/BP_Enemy` (`WidgetComponent.GetUserWidgetObject` (`self.Widget1`))))
  (bind _output_get (set `self.As BP Enemy` _asbp_enemy))
  (set `/Game/Main/UI/BP_Enemy.CurrentHealthInt` (`self.CurrenHealth`) _output_get)
  (set `/Game/Main/UI/BP_Enemy.MaxHealth` (`self.MaxHealth`) _output_get)
  (set `self.isSeeingPlayer` true)
  (`self.FollowPlayer`))

(event `self.ReceiveAnyDamage`
  (params (Damage :type "Float (single-precision)") (DamageType :type "DamageType Object Reference") (InstigatedBy :type "Controller Object Reference") (DamageCauser :type "Actor Object Reference"))
  (`KismetSystemLibrary.PrintString` (`KismetStringLibrary.Conv_DoubleToString` Damage))
  (bind _output_get (set `self.CurrenHealth` (`KismetMathLibrary.FTrunc` (- (`self.CurrenHealth`) Damage))))
  (`/Game/Main/UI/BP_Enemy.Update heath` (`self.As BP Enemy`) _output_get)
  (if (<= _output_get 0)
    (set `self.isSeeingPlayer` false)
    (`GameplayStatics.SpawnEmitterAttached` "/Game/StarterContent/Particles/P_Fire.P_Fire" (`self.CapsuleComponent`))
    (`SkeletalMeshComponent.PlayAnimation` (`self.Mesh`) "/Game/Main/Animals/Cow/Armature_Death.Armature_Death" false)
    (`PrimitiveComponent.SetCollisionEnabled` (`self.Sphere`) "NoCollision")
    (`KismetSystemLibrary.Delay` 45.0)
    (`self.K2_DestroyActor`)))

(event `self.ReceiveTick`
  (params (DeltaSeconds :type "Float (single-precision)"))
  (`KismetSystemLibrary.PrintString` "tickers")
  (if (<= (`self.CurrenHealth`) 0)
    (set `self.isSeeingPlayer` false)
    (else
      (set `self.isSeeingPlayer` true)
      (`self.FollowPlayer`))))

(event `self.PawnSensing.OnSeePawn`
  (params (Pawn :type "Pawn Object Reference"))
  (if (<= (`self.CurrenHealth`) 0)
    (`KismetSystemLibrary.PrintString` "im ded")
    (set `self.isSeeingPlayer` false)
    (`|AIMoveTo` self (`KismetMathLibrary.Conv_DoubleToVector` (`SkeletalMeshComponent.GetPosition` (`self.Mesh`))) null)
    (else
      (set `self.isSeeingPlayer` true)
      (`KismetSystemLibrary.PrintString` "isee you")
      (`self.FollowPlayer`)
      (`SkeletalMeshComponent.PlayAnimation` (`self.Mesh`) "/Game/Main/Animals/Cow/Armature_Run.Armature_Run" true)
      (if (not (`self.isSeeingPlayer`))
        (`SkeletalMeshComponent.PlayAnimation` (`self.Mesh`) "/Game/Main/Animals/Cow/Armature_Idle.Armature_Idle" false)))))

(event `FollowPlayer`
  (if (`self.isSeeingPlayer`)
    (if (not (<= (`self.CurrenHealth`) 0))
      (`|AIMoveTo` self (0.0 0.0 0.0) (`GameplayStatics.GetPlayerCharacter` 0)
        (:`then`
          (if (<= (`self.CurrenHealth`) 0)
            (set `self.isSeeingPlayer` false)
            (`|AIMoveTo` self (`KismetMathLibrary.Conv_DoubleToVector` (`SkeletalMeshComponent.GetPosition` (`self.Mesh`))) null)))))))

(fn `UserConstructionScript`)